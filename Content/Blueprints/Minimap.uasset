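; Minimap actor that toggles the first player's view to itself when M is pressed.
; An IsShowing flag picks between setting this actor as the view target and calling SetViewTargetWithBlend with no target to leave it.
; The Construction Script enables input from player controller 0, so the actor receives the key press directly.
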(event Input|KeyboardEvents|M
  (:Pressed
    (if (Variables|Default|GetIsShowing)
      (Variables|Default|SetIsShowing false)
      (Game|Player|SetViewTargetwithBlend (Game|GetPlayerController 0) 0 0.0 "VTBlend_Linear" 0.0 false)
      (else
        (Variables|Default|SetIsShowing true)
        (Game|Player|SetViewTargetwithBlend (Game|GetPlayerController 0) self 0.0 "VTBlend_Linear" 0.0 false)))))

(fn ConstructionScript
  (Input|EnableInput (Game|GetPlayerController 0)))